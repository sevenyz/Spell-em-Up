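; Magic circle actor that plays a particle effect and spawns a configurable actor at its own transform.
; The construction script applies the Color variable to the Fx component's "color" parameter, then assigns the chosen particle template.
; EnableEvent prints debug strings, passes Fx to FXX and, after a short delay, spawns ActorToSpawn.
; The Enable function is an empty stub with disconnected activate and spawn nodes.
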(event Custom|EnableEvent
  (Development|PrintString "Hello")
  (CallFunction|FXX (Variables|Default|Getfx))
  (Development|PrintString "hi")
  (Utilities|FlowControl|Delay 1.0)
  (Game|SpawnActorfromClass (Variables|Default|GetActorToSpawn) (Transformation|GetActorTransform) "Undefined" 0 0))

(fn ConstructionScript
  (|CallParentFunction)
  (Effects|Components|ParticleSystem|SetVectorParameter (Variables|Default|Getfx) "color" (Math|Conversions|ToVector(LinearColor) (Variables|Default|Getcolor)))
  (Effects|Components|ParticleSystem|SetTemplate (Variables|Default|Getfx) (Variables|Default|GetParticleSystem)))

(fn Enable)