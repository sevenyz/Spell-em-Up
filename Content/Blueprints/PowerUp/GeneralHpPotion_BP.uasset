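; GeneralHpPotion_BP is a health potion power-up base that restores HP to a player.
; HPPotionEffect takes the overlapping actor and a heal amount, then chains AddHP into SetHP.
; AddHP computes the new HP and whether it exceeds MaxHP, and SetHP writes either that sum or MaxHP, so healing never overshoots the cap.
; No overlap event or heal amount is defined here.
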(fn ConstructionScript)

(fn AddHP
  (params (Player :type Player%20Object%20Reference) (HpToAdd :type Float%20%28single-precision%29))
  (bind _currenthp (Variables|/Game/Blueprints/Player/Player.Player_C|GetCurrentHP Player))
  (bind _returnvalue (+ _currenthp HpToAdd))
  (return (> _returnvalue (Variables|/Game/Blueprints/Player/Player.Player_C|GetMaxHP Player)) _returnvalue))

(fn SetHP
  (params (Condition :type Boolean) (CurrentHP :type Float%20%28single-precision%29) (Player :type Player%20Object%20Reference))
  (if Condition
    (Variables|/Game/Blueprints/Player/Player.Player_C|SetCurrentHP Player (Variables|/Game/Blueprints/Player/Player.Player_C|GetMaxHP Player))
    (else
      (Variables|/Game/Blueprints/Player/Player.Player_C|SetCurrentHP Player CurrentHP))))

(fn HPPotionEffect
  (params (OverlappingActor :type Player%20Object%20Reference) (HpToAdd :type Float%20%28single-precision%29))
  (bind (_returnvalue _outputpin) (CallFunction|AddHP OverlappingActor HpToAdd))
  (CallFunction|SetHP _returnvalue _outputpin OverlappingActor))