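; Potion drop spawner that gives its owner a random chance to drop a health, mana, invincibility or speed potion.
; BeginPlay rolls the selector once, so the outcome is fixed before SpawnPotion is called.
; SpawnPotion switches on that roll to spawn the matching potion class at the owner's transform, with half of the possible rolls dropping nothing.
; Each result is printed as a debug string.
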(event EventBeginPlay
  (Variables|Default|SetSelector (Math|Random|RandomIntegerinRange 1 16)))

(fn SpawnPotion
  (bind _returnvalue (Components|GetOwner))
  (bind _returnvalue_2 (Transformation|GetActorTransform _returnvalue))
  (switch int (Variables|Default|GetSelector)
    (:Default
      (Development|PrintString "no drop"))
    (:1
      (bind _returnvalue_3 (Game|SpawnActorfromClass "/Game/Blueprints/PowerUp/HpPotion_S_BP.HpPotion_S_BP_C" _returnvalue_2 "Undefined" 0 0))
      (Development|PrintString (Utilities|GetDisplayName _returnvalue_3)))
    (:2
      (bind _returnvalue_4 (Game|SpawnActorfromClass "/Game/Blueprints/PowerUp/HpPotion_M_BP.HpPotion_M_BP_C" _returnvalue_2 "Undefined" 0 0))
      (Development|PrintString (Utilities|GetDisplayName _returnvalue_4)))
    (:3
      (bind _returnvalue_5 (Game|SpawnActorfromClass "/Game/Blueprints/PowerUp/HpPotion_L_BP.HpPotion_L_BP_C" _returnvalue_2 "Undefined" 0 0))
      (Development|PrintString (Utilities|GetDisplayName _returnvalue_5)))
    (:4
      (bind _returnvalue_6 (Game|SpawnActorfromClass "/Game/Blueprints/PowerUp/ManaPotion_S_BP.ManaPotion_S_BP_C" _returnvalue_2 "Undefined" 0 0))
      (Development|PrintString (Utilities|GetDisplayName _returnvalue_6)))
    (:5
      (bind _returnvalue_7 (Game|SpawnActorfromClass "/Game/Blueprints/PowerUp/ManaPotion_M_BP.ManaPotion_M_BP_C" _returnvalue_2 "Undefined" 0 0))
      (Development|PrintString (Utilities|GetDisplayName _returnvalue_7)))
    (:6
      (bind _returnvalue_8 (Game|SpawnActorfromClass "/Game/Blueprints/PowerUp/ManaPotion_L_BP.ManaPotion_L_BP_C" _returnvalue_2 "Undefined" 0 0))
      (Development|PrintString (Utilities|GetDisplayName _returnvalue_8)))
    (:7
      (bind _returnvalue_9 (Game|SpawnActorfromClass "/Game/Blueprints/PowerUp/InvincibilityPotion_BP.InvincibilityPotion_BP_C" _returnvalue_2 "Undefined" 0 0))
      (Development|PrintString (Utilities|GetDisplayName _returnvalue_9)))
    (:8
      (bind _returnvalue_10 (Game|SpawnActorfromClass "/Game/Blueprints/PowerUp/SpeedPotion_Bp.SpeedPotion_Bp_C" _returnvalue_2 "Undefined" 0 0))
      (Development|PrintString (Utilities|GetDisplayName _returnvalue_10)))))