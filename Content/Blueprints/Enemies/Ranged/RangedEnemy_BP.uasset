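; Ranged enemy that fires projectiles from a spawn point and reacts to the player's elemental attacks.
; Capsule overlaps use component tags to tell light hits (fire effect) from ranged hits (frost effect, projectile destroyed), then apply player damage and a status effect.
; Each hit charges the player's special meter and checks HP, restoring status after hit stun depending on the result.
; The SetStatus override extends the parent to toggle attacking and vulnerability during stun.
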(event OnComponentBeginOverlap(CapsuleComponent)
  (params (OverlappedComponent :type Primitive%20Component%20Object%20Reference) (OtherActor :type Actor%20Object%20Reference) (OtherComp :type Primitive%20Component%20Object%20Reference) (OtherBodyIndex :type Integer) (bFromSweep :type Boolean) (SweepResult :type Hit%20Result%20Structure%20%28by%20ref%29))
  (if (Variables|Default|GetCanBeDamaged)
    (if (Components|ComponentHasTag OtherComp "LightAttackElemental")
      (CallFunction|AttackReceivedManagement (Variables|/Game/Blueprints/Player/Player.Player_C|GetDamage (stale EventBeginPlay _output_get)) (Variables|Default|GetFireExplosion) "/Game/FXVarietyPack/Particles/P_ky_explosion.P_ky_explosion" "NewEnumerator0")
      (CallFunction|IncrementPlayerSpecialMeter (stale EventBeginPlay _output_get) (Variables|/Game/Blueprints/Player/Player.Player_C|GetCurrentSpecialMeter (stale EventBeginPlay _output_get)) 5.0)
      (bind _isdead (CallFunction|HPCheck "/Game/FXVarietyPack/Particles/P_ky_explosion.P_ky_explosion"))
      (if (Math|Boolean|Equal(Boolean) _isdead false)
        (Utilities|FlowControl|Delay (Variables|Default|GetHitStunTime))
        (CallFunction|SetStatus true (Variables|Character|GetCharacterMovement)))
      (elif (Components|ComponentHasTag OtherComp "RangedElemental")
        (Actor|DestroyActor OtherActor)
        (CallFunction|AttackReceivedManagement (Variables|/Game/Blueprints/Player/Player.Player_C|GetDamage (stale EventBeginPlay _output_get)) (Variables|Default|GetFrostExplosion) "/Game/FXVarietyPack/Particles/P_ky_waterBallHit.P_ky_waterBallHit" "NewEnumerator1")
        (CallFunction|IncrementPlayerSpecialMeter (stale EventBeginPlay _output_get) (Variables|/Game/Blueprints/Player/Player.Player_C|GetCurrentSpecialMeter (stale EventBeginPlay _output_get)) 5.0)
        (bind _isdead_2 (CallFunction|HPCheck "/Game/FXVarietyPack/Particles/P_ky_waterBallHit.P_ky_waterBallHit"))
        (if (Math|Boolean|Equal(Boolean) _isdead_2 false)
          (Utilities|FlowControl|Delay (Variables|Default|GetHitStunTime))
          (CallFunction|SetStatus true (Variables|Character|GetCharacterMovement)))))))

(event EventBeginPlay
  (bind _asplayer (Utilities|Casting|CastToPlayer (Game|GetPlayerCharacter 0))
    (:then
      (bind _output_get (Variables|Default|SetThePlayer _asplayer)))
    (:CastFailed
      (Development|PrintString "player cast fail"))))

(fn ConstructionScript
  (Variables|Default|SetHealth (Variables|Default|GetMaxHP)))

(fn Attack
  (if (Variables|Default|GetCanAttack)
    (Game|SpawnActorfromClass "/Game/Blueprints/Enemies/Ranged/ProjectileRangedEnemy.ProjectileRangedEnemy_C" (Transformation|GetWorldTransform (Variables|Default|GetProjectileSpawnPoint)) "Undefined" 0 0)))

(fn SetStatus
  (params (Status :type Boolean) (CharacterMovement :type Actor%20Component%20Object%20Reference))
  (bind _statusset (|CallParentFunction Status CharacterMovement))
  (Variables|Default|SetCanBeDamaged Status)
  (Variables|Default|SetCanAttack Status)
  (return _statusset))

(fn AttackReceivedManagement
  (params (Damage :type Float%20%28single-precision%29) (ParticleEffectHit :type Actor%20Component%20Object%20Reference) (ParticleEffectDeath :type Particle%20System%20Object%20Reference) (StatusEffect :type StatusEffects_Enemy%20Enum :default "NewEnumerator0"))
  (CallFunction|SetStatus false (Variables|Character|GetCharacterMovement))
  (Variables|Default|SetStatusEffects StatusEffect)
  (CallFunction|ApplyDamage Damage)
  (CallFunction|GSetStatusEffect)
  (Components|Activation|Activate ParticleEffectHit false))