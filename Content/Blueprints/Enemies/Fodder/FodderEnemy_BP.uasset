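; Fodder enemy that takes elemental hits from the player and damages and stuns the player through an overlap-box attack.
; Capsule overlaps use component tags to tell light from ranged hits, then apply damage, status and particles and charge the player's special meter.
; SetStatus switches off damageability and attacking during hit stun, extending a parent version.
; A looping timer drives a short burn damage-over-time effect.
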(event OnComponentBeginOverlap(CapsuleComponent)
  (params (OverlappedComponent :type Primitive%20Component%20Object%20Reference) (OtherActor :type Actor%20Object%20Reference) (OtherComp :type Primitive%20Component%20Object%20Reference) (OtherBodyIndex :type Integer) (bFromSweep :type Boolean) (SweepResult :type Hit%20Result%20Structure%20%28by%20ref%29))
  (if (Variables|Default|GetCanBeDamaged)
    (if (Components|ComponentHasTag OtherComp "LightAttackElemental")
      (CallFunction|AttackReceivedManagement (Variables|Default|GetFireExplosion) "/Game/FXVarietyPack/Particles/P_ky_explosion.P_ky_explosion" (Variables|/Game/Blueprints/Player/Player.Player_C|GetDamage (stale EventBeginPlay _output_get)) "NewEnumerator0")
      (CallFunction|IncrementPlayerSpecialMeter (stale EventBeginPlay _output_get) (Variables|/Game/Blueprints/Player/Player.Player_C|GetCurrentSpecialMeter (stale EventBeginPlay _output_get)) 5.0)
      (Utilities|FlowControl|Delay (Variables|Default|GetHitStunTime))
      (CallFunction|SetStatus true (Variables|Character|GetCharacterMovement))
      (elif (Components|ComponentHasTag OtherComp "RangedElemental")
        (CallFunction|AttackReceivedManagement (Variables|Default|GetFrostExplosion) "/Game/FXVarietyPack/Particles/P_ky_waterBallHit.P_ky_waterBallHit" (Variables|/Game/Blueprints/Player/Player.Player_C|GetDamage (stale EventBeginPlay _output_get)) "NewEnumerator7")
        (CallFunction|IncrementPlayerSpecialMeter (stale EventBeginPlay _output_get) (Variables|/Game/Blueprints/Player/Player.Player_C|GetCurrentSpecialMeter (stale EventBeginPlay _output_get)) 1e+01)
        (Utilities|IsValid self
          (:Is%20Valid
            (Actor|DestroyActor OtherActor)
            (Utilities|FlowControl|Delay (Variables|Default|GetHitStunTime))
            (CallFunction|SetStatus true (Variables|Character|GetCharacterMovement))))))))

(event EventBeginPlay
  (bind _asplayer (Utilities|Casting|CastToPlayer (Game|GetPlayerCharacter 0))
    (:then
      (bind _output_get (Variables|Default|SetThePlayer _asplayer)))
    (:CastFailed
      (Development|PrintString "player cast fail"))))

(fn ConstructionScript
  (Variables|Default|SetHealth (Variables|Default|GetMaxHP)))

(fn Attack
  (bind _theplayer (Variables|Default|GetThePlayer))
  (if (and (Variables|Default|GetCanAttack) (Collision|IsOverlappingActor (Variables|Default|GetAttackBox) _theplayer :!class /Script/Engine.PrimitiveComponent))
    (Components|Activation|Activate (Variables|Default|GetAttackEffect) false)
    (Default|IsHitEvent _theplayer (Variables|Default|GetAttackDamage) (Variables|Default|GetAttackStunTime))
    (Effects|SpawnEmitterAttached "/Game/FXVarietyPack/Particles/P_ky_shotShockwave.P_ky_shotShockwave" (Variables|/Script/Paper2D.PaperCharacter|GetSprite _theplayer) "None")))

(fn SetStatus
  (params (CanDoStuff :type Boolean))
  (Variables|Default|SetCanBeDamaged CanDoStuff)
  (Variables|Default|SetCanAttack CanDoStuff)
  (Components|Activation|SetActive (Variables|Character|GetCharacterMovement) CanDoStuff false)
  (return))

(fn ApplyDamage
  (bind _output_get (Variables|Default|SetMaxHP (- (Variables|Default|GetMaxHP) (Variables|/Game/Blueprints/Player/Player.Player_C|GetDamage (Variables|Default|GetThePlayer)))))
  (return _output_get))

(fn HpCheck
  (if (<= (Variables|Default|GetMaxHP) 0.0)
    (Actor|DestroyActor)))

(fn AttackReceivedManagement
  (params (ParticleEffectHit :type Actor%20Component%20Object%20Reference) (ParticleEffectDeath :type Particle%20System%20Object%20Reference) (Damage :type Float%20%28single-precision%29) (StatusEffect :type StatusEffects_Enemy%20Enum :default "NewEnumerator0"))
  (CallFunction|SetStatus false (Variables|Character|GetCharacterMovement))
  (Variables|Default|SetStatusEffects StatusEffect)
  (CallFunction|ApplyDamage Damage)
  (CallFunction|GSetStatusEffect)
  (Components|Activation|Activate ParticleEffectHit false)
  (CallFunction|HPCheck))

(fn SetStatus
  (params (Status :type Boolean) (CharacterMovement :type Actor%20Component%20Object%20Reference))
  (bind _statusset (|CallParentFunction Status CharacterMovement))
  (Variables|Default|SetCanBeDamaged Status)
  (Variables|Default|SetCanAttack Status)
  (return _statusset))

(fn BurnEffect
  (if (<= (Utilities|Time|GetTimeSeconds) (+ (Variables|Default|GetTimeBeforeDot) 3.0))
    (CallFunction|ApplyDamage 2.0)
    (Development|PrintString (Utilities|String|ToString(Float) (Variables|Default|GetHealth)))
    (CallFunction|HPCheck)
    (CallFunction|GSpawnDeathParticle "/Game/FXVarietyPack/Particles/P_ky_explosion.P_ky_explosion" "0.500000,0.500000,0.500000")
    (else
      (Utilities|Time|ClearTimerbyFunctionName 0 "BurnEffect"))))

(fn SetBurnEffect
  (Variables|Default|SetTimeBeforeDot (Utilities|Time|GetTimeSeconds))
  (Utilities|Time|SetTimerbyFunctionName 0 "BurnEffect" 1.0 true))