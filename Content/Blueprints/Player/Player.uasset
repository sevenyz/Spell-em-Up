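; Player character with flipbook sprites and clamped-depth movement, handling HP, regenerating mana, potions, stun, death and pausing.
; BeginPlay spawns Elemental and Necromancy tomes from the SelectedTomes map, and a FlipFlop input switches between them.
; Light and ranged attacks check Elemental mana costs, then run a cast delay that hits cancel.
; Elemental attacks spawn hitboxes or projectiles, and its meter-gated special damages enemies inside the camera trigger; Necromancy only forwards calls.
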(event Custom|IsHitEvent
  (params (Damage :type Float%20%28single-precision%29) (StunTime :type Float%20%28single-precision%29))
  (bind _sprite (Variables|Default|GetSprite))
  ;[1 1 1] IsHitEvent
  (if (Variables|Default|GetIsInvincible)
    (Variables|Default|SetIsInvincible false)
    (else
      (Components|Activation|SetActive (Variables|Default|GetFireCast) false false)
      (Components|Activation|SetActive (Variables|Default|GetGlacialCast) false false)
      (Variables|Default|SetIsHit true)
      (Variables|Default|SetCurrentHP (- (Variables|Default|GetCurrentHP) Damage))
      (if (CallFunction|CheckHP)
        (Default|CallDeathDispatcher)
        (Input|DisableInput 0)
        (else
          (switch Utilities|FlowControl|Switch|SwitchonDirection (Variables|Default|GetDirection)
            (:NewEnumerator2
              (Sprite|SetFlipbook _sprite "/Game/Sprites/Player_Test/Stunned_Left/player_stunned_left_flipbook.player_stunned_left_flipbook"))
            (:NewEnumerator3
              (Sprite|SetFlipbook _sprite "/Game/Sprites/Player_Test/Stunned_Right/player_stunned_right_flipbook.player_stunned_right_flipbook")))
          (Input|DisableInput 0)
          (Utilities|FlowControl|Delay StunTime)
          (Sprite|SetFlipbook (Variables|Default|GetSprite) (Utilities|Select :Index (Variables|Default|GetDirection) :NewEnumerator2 "/Game/Sprites/Link/Link_Idle_Left.Link_Idle_Left" :NewEnumerator3 "/Game/Sprites/Link/Link_Idle_Right.Link_Idle_Right"))
          (Input|EnableInput (Game|GetPlayerController 0)))))))

(event Custom|ManaPotionEvent
  ;[0 0.4289 1] ManaPotionEvent
  (Variables|Default|SetCurrentMana 9999999.0)
  (Utilities|FlowControl|Delay (Variables|Default|GetManaPotionTime))
  (Variables|Default|SetCurrentMana (Variables|Default|GetMaxMana)))

(event Custom|SpeedPotionEvent
  ;[1 1 1] SpeedPotionEvent
  (Variables|/Script/Engine.CharacterMovementComponent|SetMaxWalkSpeed (Variables|Character|GetCharacterMovement) 4.5e+02))

(event EventBeginPlay
  (Variables|Default|SetCurrentMana (Variables|Default|GetMaxMana))
  (Variables|Default|SetCurrentHP (Variables|Default|GetMaxHP))
  (Utilities|Time|SetTimerbyFunctionName 0 "RestoreMana" 0.5 true)
  (bind _values (Utilities|Map|Values (Variables|Default|GetSelectedTomes)))
  (bind _index (CallFunction|GetMapValue (Utilities|Array|Length _values) _values))
  (bind _tome (CallFunction|GetTomeClass _index))
  (bind _aselemental_tome (Utilities|Casting|CastToElementalTomeClass _tome))
  (bind _returnvalue (Game|SpawnActorfromClass _aselemental_tome (Transformation|GetActorTransform) "Undefined" 0 0))
  (Variables|Default|SetElementalTome _returnvalue)
  (Utilities|Array|SetArrayElem _values _index false)
  (bind _index_2 (CallFunction|GetMapValue (Utilities|Array|Length _values) _values))
  (bind _tome_2 (CallFunction|GetTomeClass _index_2))
  (bind _asnecromancy_tome (Utilities|Casting|CastToNecromancyTomeClass _tome_2))
  (bind _returnvalue_2 (Game|SpawnActorfromClass _asnecromancy_tome (Transformation|GetActorTransform) "Undefined" 0 0))
  (Variables|Default|SetNecromancyTome _returnvalue_2)
  (Utilities|Array|SetArrayElem _values _index_2 false)
  (bind _outactors (Actor|GetAllActorsOfClass "/Game/CameraActor_BP.CameraActor_BP_C"))
  (Variables|Default|SetCameraObj (Utilities|Array|Get(acopy) _outactors)))

(event Input|ActionEvents|InputActionPauseGame
  (params (Key :type Key%20Structure))
  ;[0.6128 0.1171 0.726] Pause Game
  (:Pressed
    (CallFunction|PauseGame)))

(event Input|ActionEvents|InputActionLightAttack
  (params (Key :type Key%20Structure))
  ;[1 1 1] LightAttack
  (:Pressed
    (bind _hasenoughmana (CallFunction|CheckMana (Variables|/Game/Blueprints/Tomes/GenericTome.GenericTome_C|GetLightAttackManaCost (Variables|Default|GetElementalTome))))
    (if _hasenoughmana
      (CallFunction|AttackCastManagement (Variables|Default|GetFireCast))
      (Utilities|FlowControl|Delay (Variables|Default|GetLightAttackCastTime))
      (bind _canattack (CallFunction|AttackInitialization (Variables|Default|GetFireCast)))
      (if _canattack
        (if (Variables|Default|GetIsFirstTome)
          (bind _damage (Default|LightAttack (Variables|Default|GetElementalTome)))
          ;;[1 1 1] Active
          (Variables|Default|SetDamage _damage)
          (bind _returnvalue (Game|SpawnActorfromClass "/Game/Blueprints/Player/LightAttackTest.LightAttackTest_C" (Transformation|GetWorldTransform (Variables|Default|GetLightAttackPos)) "Undefined" 0 0))
          ;;[1 1 1] Recovery
          (Utilities|FlowControl|Delay 0.5)
          (Actor|DestroyActor _returnvalue)
          (Input|EnableInput 0)
          (else
            (Default|LightAttack (Variables|Default|GetNecromancyTome)))))
      (else
        (Development|PrintString "not enough mana" true true "(R=1.000000,G=0.000000,B=0.000000,A=1.000000)")))))

(event Input|ActionEvents|InputActionRangedAttack
  (params (Key :type Key%20Structure))
  ;[1 1 1] RangedAttack
  (:Pressed
    (bind _hasenoughmana (CallFunction|CheckMana (Variables|/Game/Blueprints/Tomes/GenericTome.GenericTome_C|GetRangedAttackManaCost (Variables|Default|GetElementalTome))))
    (if _hasenoughmana
      (CallFunction|AttackCastManagement (Variables|Default|GetGlacialCast))
      (Utilities|FlowControl|Delay (Variables|Default|GetRangedAttackCastTime))
      (bind _canattack (CallFunction|AttackInitialization (Variables|Default|GetGlacialCast)))
      (if _canattack
        (if (Variables|Default|GetIsFirstTome)
          (bind _damage (Default|RangedAttack (Variables|Default|GetElementalTome)))
          (Variables|Default|SetDamage _damage)
          (Game|SpawnActorfromClass "/Game/Blueprints/Player/ProjectileTest.ProjectileTest_C" (Transformation|GetWorldTransform (Variables|Default|GetSpellSpawnPoint)) "Undefined" 0 0)
          (Utilities|FlowControl|Delay 0.5)
          (Input|EnableInput 0)
          (else
            (Default|RangedAttack (Variables|Default|GetNecromancyTome)))))
      (else
        (Development|PrintString "not enough mana")))))

(event Input|ActionEvents|InputActionSpecialAttack
  (params (Key :type Key%20Structure))
  (bind _cameraobj (Variables|Default|GetCameraObj))
  (bind _particlesystem (Variables|/Game/CameraActor_BP.CameraActor_BP_C|GetParticleSystem _cameraobj))
  ;[1 1 1] SpecialAttack
  (:Pressed
    (if (>= (Variables|Default|GetCurrentSpecialMeter) (Variables|Default|GetMaxSpecialMeter))
      (if (Variables|Default|GetIsFirstTome)
        (Default|SpecialAttack (Variables|Default|GetElementalTome))
        (Input|DisableInput 0)
        (Variables|/Script/Engine.MovementComponent|SetVelocity (Variables|Character|GetCharacterMovement) "0, 0, 0")
        (Variables|Default|SetCurrentSpecialMeter 0.0)
        (bind _output_get (Variables|Default|SetCameraOverlappingActors (Collision|GetOverlappingActors (Variables|/Game/CameraActor_BP.CameraActor_BP_C|GetCameraTrigger _cameraobj) "/Game/Blueprints/Enemies/GeneralEnemy/GeneralEnemy.GeneralEnemy_C" :!class /Script/Engine.PrimitiveComponent)))
        (Components|Activation|ToggleActive _particlesystem)
        (Utilities|FlowControl|Delay 1.0)
        (for _array_element _output_get
          (bind _asgeneral_enemy (Utilities|Casting|CastToGeneralEnemy _array_element))
          (Default|ApplyDamage _asgeneral_enemy 3e+01)
          (Default|HPCheck _asgeneral_enemy "/Game/FXVarietyPack/Particles/P_ky_shotShockwave.P_ky_shotShockwave"))
        (Utilities|FlowControl|Delay 0.5)
        (Components|Activation|ToggleActive _particlesystem)
        (Input|EnableInput 0)
        (else
          (Default|SpecialAttack (Variables|Default|GetNecromancyTome)))))))

(event Input|ActionEvents|InputActionTomeSwitch
  (params (Key :type Key%20Structure))
  ;[1 1 1] TomeSwitch
  (:Pressed
    (Utilities|FlowControl|FlipFlop
      (:A
        (Variables|Default|SetIsFirstTome false))
      (:B
        (Variables|Default|SetIsFirstTome true)))))

(event Input|AxisEvents|InputAxisXAxis
  (params (AxisValue :type Float%20%28single-precision%29))
  (bind _cube (Variables|Default|GetCube))
  (CallFunction|SetDirection)
  (if (Utilities|Enum|Equal(Enum) (Variables|Default|GetDirection) "NewEnumerator3")
    (Transformation|SetRelativeRotation _cube (Math|Rotator|MakeRotator 0.0 0.0 -9e+01) false false)
    (else
      (Transformation|SetRelativeRotation _cube (Math|Rotator|MakeRotator 0.0 0.0 9e+01) false false)))
  (Pawn|Input|AddMovementInput "0.000000,-1.000000, 0" AxisValue false))

(event Input|AxisEvents|InputAxisYAxis
  (params (AxisValue :type Float%20%28single-precision%29))
  (CallFunction|YAxisClamp)
  (Pawn|Input|AddMovementInput "-1.000000,0.000000, 0" AxisValue false))

(fn ConstructionScript)

(fn SetDirection
  (if (Utilities|IsPlayerMoving)
    (Variables|Default|SetDirection (Utilities|DirectionSetup)))
  (Sprite|SetFlipbook (Variables|Default|GetSprite) (select (> (Math|Vector|VectorLength (Transformation|GetVelocity)) 0.0) (Utilities|Select :Index (Variables|Default|GetDirection) :NewEnumerator2 "/Game/Sprites/Player_Test/Idle_Left/player_idle_left_flipbook.player_idle_left_flipbook" :NewEnumerator3 "/Game/Sprites/Player_Test/Idle_right/player_idle_right_flipbook.player_idle_right_flipbook") (Utilities|Select :Index (Variables|Default|GetDirection) :NewEnumerator2 "/Game/Sprites/Player_Test/Idle_Left/player_idle_left_flipbook.player_idle_left_flipbook" :NewEnumerator3 "/Game/Sprites/Player_Test/Idle_right/player_idle_right_flipbook.player_idle_right_flipbook"))))

(fn YAxisClamp
  (bind _returnvalue (Transformation|GetActorLocation))
  (if (>= (.x _returnvalue) 4.5e+02)
    (Transformation|SetActorLocation (Math|Vector|MakeVector 4.5e+02 (.y _returnvalue) (.z _returnvalue)) false false)
    (elif (<= (.x _returnvalue) -4.5e+02)
      (Transformation|SetActorLocation (Math|Vector|MakeVector -4.5e+02 (.y _returnvalue) (.z _returnvalue)) false false))))

(fn RestoreMana
  (if (< (Variables|Default|GetCurrentMana) (Variables|Default|GetMaxMana))
    (Variables|Default|SetCurrentMana (+ (Variables|Default|GetCurrentMana) 2.0))))

(fn GetMapValue
  (params (LastIndex :type Integer) (Array :type Array%20of%20Booleans))
  ;[1 1 1] Gets for the first TRUE value in the map
  (bind _index (Utilities|FlowControl|ForLoopwithBreak 0 LastIndex :!label _label)
    (:LoopBody
      (if (Utilities|Array|Get(acopy) Array _index)
        (goto _label Break)))
    (:Completed
      (return _index))))

(fn GetTomeClass
  (params (Index :type Integer))
  ;[1 1 1] Gets the tome of the corresponding index in the map
  (bind _keys (Utilities|Map|Keys (Variables|Default|GetSelectedTomes)))
  (return (Utilities|Array|Get(acopy) _keys Index)))

(fn PauseGame
  (bind _returnvalue (Game|GetPlayerController 0))
  (Game|SetGamePaused true)
  (Utilities|IsValid (Variables|Default|GetPauseMenu)
    (:Is%20Valid
      _)
    (:Is%20Not%20Valid
      (bind _returnvalue_2 (UserInterface|CreateWidget "/Game/UI/PauseMenu.PauseMenu_C" (Game|GetPlayerController 0)))
      (Variables|Default|SetPauseMenu _returnvalue_2)))
  (UserInterface|Viewport|AddtoViewport (Variables|Default|GetPauseMenu) 0)
  (Input|SetInputModeUIOnly _returnvalue (Variables|Default|GetPauseMenu) "DoNotLock")
  (Variables|/Script/Engine.PlayerController|SetbShowMouseCursor _returnvalue true))

(fn UnpauseGame
  (bind _returnvalue (Game|GetPlayerController 0))
  (Game|SetGamePaused false)
  (Widget|RemovefromParent (Variables|Default|GetPauseMenu))
  (Input|SetInputModeGameOnly _returnvalue)
  (Variables|/Script/Engine.PlayerController|SetbShowMouseCursor _returnvalue false))

(fn CheckHP
  (return (<= (Variables|Default|GetCurrentHP) 0.0)))

(fn AttackCastManagement
  (params (CastEffect :type Actor%20Component%20Object%20Reference))
  (Variables|Default|SetIsHit false)
  (Input|DisableInput (Game|GetPlayerController 0))
  (Variables|/Script/Engine.MovementComponent|SetVelocity (Variables|Character|GetCharacterMovement) "0, 0, 0")
  (Components|Activation|SetActive CastEffect true false))

(fn AttackInitialization
  (params (AttackEffect :type Actor%20Component%20Object%20Reference))
  (if (Variables|Default|GetIsHit)
    (return false)
    (else
      (Components|Activation|SetActive AttackEffect false false)
      (Input|EnableInput 0)
      (return true))))

(fn CheckMana
  (params (ManaNeeded :type Float%20%28single-precision%29))
  (return (< ManaNeeded (Variables|Default|GetCurrentMana))))