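; NecromancyTome is a child tome Blueprint that defines the necromancy variant of the light, ranged, grab and special attacks.
; Each override runs the parent attack, prints a debug string and returns the parent's result.
; Light, ranged and grab attacks also set EnemyStatusEffects to a different enum value each, after the parent call.
; The special attack adds only the debug print.
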(fn ConstructionScript
  (|CallParentFunction))

(fn LightAttack
  (bind _damage (|CallParentFunction))
  (Variables|Default|SetEnemyStatusEffects "NewEnumerator3")
  (Development|PrintString "Necro light")
  (return _damage))

(fn RangedAttack
  (bind _damage (|CallParentFunction))
  (Variables|Default|SetEnemyStatusEffects "NewEnumerator4")
  (Development|PrintString "Necro ranged")
  (return _damage))

(fn GrabAttack
  (bind _damage (|CallParentFunction))
  (Variables|Default|SetEnemyStatusEffects "NewEnumerator11")
  (Development|PrintString "Necro grab")
  (return _damage))

(fn SpecialAttack
  (bind _damage (|CallParentFunction))
  (Development|PrintString "Necro special")
  (return _damage))