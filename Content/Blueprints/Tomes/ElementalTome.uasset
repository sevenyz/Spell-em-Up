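; Elemental tome, a child Blueprint that overrides the light, ranged, grab and special attacks of its parent.
; Each override runs the parent attack, prints a debug string and returns the parent's result.
; Light, ranged and grab also set EnemyStatusEffects to a different enum value each after the parent call.
; The special attack leaves the status effect unchanged.
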(fn ConstructionScript
  (|CallParentFunction))

(fn LightAttack
  (bind _damage (|CallParentFunction))
  (Variables|Default|SetEnemyStatusEffects "NewEnumerator0")
  (Development|PrintString "Elemental light")
  (return _damage))

(fn RangedAttack
  (bind _damage (|CallParentFunction))
  (Variables|Default|SetEnemyStatusEffects "NewEnumerator1")
  (Development|PrintString "Elemental ranged")
  (return _damage))

(fn GrabAttack
  (bind _damage (|CallParentFunction))
  (Variables|Default|SetEnemyStatusEffects "NewEnumerator2")
  (Development|PrintString "Elemental grab")
  (return _damage))

(fn SpecialAttack
  (bind _damage (|CallParentFunction))
  (Development|PrintString "Elemental special")
  (return _damage))