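; GenericTome is a tome Blueprint that supplies light, ranged, grab and special attack damage for the player.
; On BeginPlay it casts and caches the player character so attacks can subtract their mana cost from the player's CurrentMana.
; Light, ranged and grab attacks set a priority flag, true only for ranged, then spend mana and return damage.
; SpecialAttack only returns its damage, with no mana cost.
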(event EventBeginPlay
  (bind _asplayer (Utilities|Casting|CastToPlayer (Game|GetPlayerCharacter 0))
    (:then
      (Variables|Default|SetPlayer _asplayer))
    (:CastFailed
      (Development|PrintString "cast failed"))))

(fn ConstructionScript)

(fn LightAttack
  (Variables|Default|SetHasHighPriority false)
  (CallFunction|DecreaseMana (Variables|Default|GetLightAttackManaCost))
  (return (Variables|Default|GetLightAttackDamage)))

(fn RangedAttack
  (Variables|Default|SetHasHighPriority true)
  (CallFunction|DecreaseMana (Variables|Default|GetRangedAttackManaCost))
  (return (Variables|Default|GetRangedAttackDamage)))

(fn GrabAttack
  (Variables|Default|SetHasHighPriority false)
  (CallFunction|DecreaseMana (Variables|Default|GetGrabAttackManaCost))
  (return (Variables|Default|GetGrabAttackDamage)))

(fn SpecialAttack
  (return (Variables|Default|GetSpecialAttackDamage)))

(fn DecreaseMana
  (params (ManaCost :type Float%20%28single-precision%29))
  (bind _player (Variables|Default|GetPlayer))
  (Variables|/Game/Blueprints/Player/Player.Player_C|SetCurrentMana _player (- (Variables|/Game/Blueprints/Player/Player.Player_C|GetCurrentMana _player) ManaCost)))